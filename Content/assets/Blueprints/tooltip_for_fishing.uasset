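; Trigger actor that shows a fishing tooltip widget on screen when an actor overlaps it.
; The Check flag gates the begin-overlap event and is cleared on display, so the tooltip is created only once.
; The widget is stored in NewVar0 and removed after a short delay or when an overlap ends.
; Neither event filters which actor overlaps.
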(event EventBeginPlay)

(event Collision|EventActorBeginOverlap
  (params (OtherActor :type Actor%20Object%20Reference))
  (if (Variables|Default|Getcheck)
    (bind _returnvalue (UserInterface|CreateWidget "/Game/assets/widget/tooltip_For_fishing_widget.tooltip_For_fishing_widget_C"))
    (Variables|Default|SetNewVar_0 _returnvalue)
    (UserInterface|Viewport|AddtoViewport _returnvalue 0)
    (Variables|Default|Setcheck false)
    (Utilities|FlowControl|Delay 3.0)
    (Widget|RemovefromParent (Variables|Default|GetNewVar_0))))

(event EventTick
  (params (DeltaSeconds :type Float%20%28single-precision%29)))

(event Collision|EventActorEndOverlap
  (params (OtherActor :type Actor%20Object%20Reference))
  (Widget|RemovefromParent (Variables|Default|GetNewVar_0)))

(fn ConstructionScript)