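; A trigger box Blueprint that exchanges the player's fish for coins.
; On overlap by the ThirdPersonCharacter, it calls CheckInventory, spawns one Coin at the Coinspawn actor's transform for each point of Fishing, then resets that count to zero.
; With no fish, it shows a NotenoughfishWBP widget for a short delay before removing it.
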(event EventBeginPlay
  (if true
    _))

(event Collision|EventActorBeginOverlap
  (params (OtherActor :type Actor%20Object%20Reference))
  (bind _asthird_person_character (Utilities|Casting|CastToThirdPersonCharacter OtherActor))
  (Default|CheckInventory _asthird_person_character)
  (if (>= (Variables|/Game/assets/Blueprints/ThirdPersonCharacter.ThirdPersonCharacter_C|Getfishing _asthird_person_character) 1)
    (for _index (range 1 (Variables|/Game/assets/Blueprints/ThirdPersonCharacter.ThirdPersonCharacter_C|Getfishing _asthird_person_character))
      (Game|SpawnActorfromClass "/Game/assets/Blueprints/coin.coin_C" (Transformation|GetActorTransform (Variables|Default|Getcoinspawn)) "AdjustIfPossibleButAlwaysSpawn" 0 0))
    (Variables|/Game/assets/Blueprints/ThirdPersonCharacter.ThirdPersonCharacter_C|Setfishing _asthird_person_character 0)
    (else
      (bind _returnvalue (UserInterface|CreateWidget "/Game/assets/widget/notenoughfishWBP.notenoughfishWBP_C"))
      (bind _output_get (Variables|Default|Settext _returnvalue))
      (UserInterface|Viewport|AddtoViewport _returnvalue 0)
      (Utilities|FlowControl|Delay 2.0)
      (Widget|RemovefromParent _output_get))))

(event EventTick
  (params (DeltaSeconds :type Float%20%28single-precision%29)))

(fn ConstructionScript)